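; Main game mode for a local multiplayer game in which players control BP_Ghost pawns.
; On begin play it caches the ghosts and game state manager, then, after a one-tick delay, creates a local player for each connected input device lacking a player controller.
; StartGame sets the playing flag and forwards to the state manager.
; A separate event spawns a ghost at a player start and possesses it with a given controller.
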(event `self.ReceiveBeginPlay`
  ;[1 0 0] Begin Play
  (`|ExecutionSequence`
    (:`then_0`
      ;[0.2396 0.1641 0.07344] Fetch references in scene
      (bind _outactors (`GameplayStatics.GetAllActorsOfClass` "/Game/Blueprints/Ghost/BP_Ghost.BP_Ghost_C"))
      (set `self.Ghost Pawns` _outactors)
      (bind _returnvalue (`GameplayStatics.GetActorOfClass` "/Game/Blueprints/Game/BP_GameStateManager.BP_GameStateManager_C"))
      (set `self.Game State` _returnvalue))
    (:`then_1`
      ;[0.03992 0.08123 0.1198] For each connected gamepad
      (`KismetSystemLibrary.DelayUntilNextTick`)
      (bind _outusers (`InputDeviceLibrary.GetAllActiveUsers`))
      (for _array_element _outusers
        (bind _returnvalue_2 (`InputDeviceLibrary.GetPrimaryInputDeviceForUser` _array_element))
        (`KismetSystemLibrary.PrintString` (`KismetStringLibrary.Conv_PlatformUserIdToString` _array_element))
        (bind _returnvalue_3 (`InputDeviceLibrary.GetInputDeviceConnectionState` _returnvalue_2))
        (if (`|EnumEquality` _returnvalue_3 "Connected")
          (`/Engine/EditorBlueprintResources/StandardMacros.IsValid` (`GameplayStatics.GetPlayerControllerFromPlatformUser` _array_element)
            (:`Is Not Valid`
              ;[1 0.415 0.1828] create a new player controller if needed
              (bind _asgame_mode_main (cast `/Game/Blueprints/GameMode/GameMode_Main` (`GameplayStatics.GetGameMode`)))
              (`self.CreateNewPlayer` _asgame_mode_main)))
          (else
            (`KismetSystemLibrary.PrintString` "not connected")))))))

(event `StartGame`
  ;[1 0.05092 0.03103] Start Game
  (set `self.IsPlaying` true)
  (`/Game/Blueprints/Game/BP_GameStateManager.StartGame` (`self.Game State`)))

(event `CreateNewPlayer`
  ;[0.04395 0.1972 0.3438 0.856] Create new Player Controller
  (`KismetSystemLibrary.PrintString` "new player")
  (`GameplayStatics.CreatePlayer` -1)
  (bind _outactors (`GameplayStatics.GetAllActorsOfClass` "/Game/Blueprints/Ghost/BP_Ghost.BP_Ghost_C"))
  (set `self.Ghost Pawns` _outactors))

(event `Spawn and possess ghost`
  (params (`player controller` :type "PlayerController Object Reference"))
  ;[0.2407 0.5669 0.6927 0.877] Create new Ghost Pawn
  (bind _returnvalue (`|SpawnActorFromClass` "/Game/Blueprints/Ghost/BP_Ghost.BP_Ghost_C" (`self.GetTransform` (`self.K2_FindPlayerStart` null)) "AdjustIfPossibleButAlwaysSpawn" "MultiplyWithRoot" null null))
  (`Controller.Possess` `player controller` _returnvalue))

(fn `UserConstructionScript`)