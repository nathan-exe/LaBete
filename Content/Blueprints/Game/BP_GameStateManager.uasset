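; Game state manager Blueprint that hosts the coin, ghost, power, timer, win and windows managers as child actors and starts the game.
; On BeginPlay it casts each child actor and caches a typed reference to it.
; StartGame runs once, guarded by a GameStarted flag, refreshing the ghost list and starting the timer.
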(event `self.ReceiveBeginPlay`
  (`self.Setup Child Ref`))

(event `StartGame`
  (if (not (`self.GameStarted`))
    (`/Game/Blueprints/Ghost/BP_GhostManager.Update Ghost List` (`self.GhostManagerRef`))
    (`/Game/Blueprints/Timer/BP_TimerManager.StartTimer` (`self.TimerManagerRef`))
    (set `self.GameStarted` true)))

(fn `Setup Child Ref`
  (bind _asbp_coin_manager (cast `/Game/Blueprints/Coin/BP_CoinManager` (`ChildActorComponent.ChildActor` (`self.BP_CoinManager`))))
  (set `self.CoinManagerRef` _asbp_coin_manager)
  (bind _asbp_ghost_manager (cast `/Game/Blueprints/Ghost/BP_GhostManager` (`ChildActorComponent.ChildActor` (`self.BP_GhostManager`))))
  (set `self.GhostManagerRef` _asbp_ghost_manager)
  (bind _asbp_power_manager (cast `/Game/Blueprints/Power/BP_PowerManager` (`ChildActorComponent.ChildActor` (`self.BP_PowerManager`))))
  (set `self.PowerManagerRef` _asbp_power_manager)
  (bind _asbp_timer_manager (cast `/Game/Blueprints/Timer/BP_TimerManager` (`ChildActorComponent.ChildActor` (`self.BP_TimerManager`))))
  (set `self.TimerManagerRef` _asbp_timer_manager)
  (bind _asbp_win_manager (cast `/Game/Blueprints/Win/BP_WinManager` (`ChildActorComponent.ChildActor` (`self.BP_WinManager`))))
  (set `self.WinManagerRef` _asbp_win_manager)
  (bind _asbp_windows_manager (cast `/Game/Blueprints/Windows/BP_WindowsManager` (`ChildActorComponent.ChildActor` (`self.BP_WindowsManager`))))
  (set `self.WindowsManagerRef` _asbp_windows_manager))

(fn `UserConstructionScript`)