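; BP_DebugComponent provides debug events that manually trigger window, coin and power spawns in the game.
; On BeginPlay it finds the BP_GameStateManager actor and caches a reference to it.
; Each DEBUG_ event reaches the matching window, coin or power manager through that reference and calls its spawn function.
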(event `self.ReceiveBeginPlay`
  (bind _returnvalue (`GameplayStatics.GetActorOfClass` "/Game/Blueprints/Game/BP_GameStateManager.BP_GameStateManager_C"))
  (set `self.GameManagerRef` _returnvalue))

(event `DEBUG_SpawnWindow`
  (`/Game/Blueprints/Windows/BP_WindowsManager.SpawnWindow` (`/Game/Blueprints/Game/BP_GameStateManager.WindowsManagerRef` (`self.GameManagerRef`))))

(event `DEBUG_SpawnCoin`
  (`/Game/Blueprints/Coin/BP_CoinManager.SpawnCoin` (`/Game/Blueprints/Game/BP_GameStateManager.CoinManagerRef` (`self.GameManagerRef`))))

(event `DEBUG_SpawnPower`
  (`/Game/Blueprints/Power/BP_PowerManager.SpawnPower` (`/Game/Blueprints/Game/BP_GameStateManager.PowerManagerRef` (`self.GameManagerRef`))))