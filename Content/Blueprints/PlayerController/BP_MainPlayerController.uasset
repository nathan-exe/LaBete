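; Main player controller that configures the top-down camera and switches Enhanced Input mappings to match the possessed pawn.
; On possession, a local controller calls SetupCam on the top-down camera manager, then adds the mapping context for a turret, spectator or ghost pawn, chosen by cast.
; On unpossession, it removes the matching context, without the local-controller check.
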(event `self.ReceivePossess`
  (params (PossessedPawn :type "Pawn Object Reference"))
  (bind _returnvalue (pcsubsystem `EnhancedInputLocalPlayerSubsystem` self))
  ;[1 0.03429 0] Possessed Pawn
  (if (`self.IsLocalController`)
    (`|ExecutionSequence`
      (:`then_0`
        ;[0.731 0.4324 0.3666 0.697] Setup Camera
        (bind _asbp_top_down_cam_manager (cast `/Game/Blueprints/Cam/BP_TopDown_CamManager` (`GameplayStatics.GetPlayerCameraManager` 0)))
        (`/Game/Blueprints/Cam/BP_TopDown_CamManager.SetupCam` _asbp_top_down_cam_manager))
      (:`then_1`
        ;[0.03737 0.07216 0.151 0.769] Setup input context for possessed pawn
        (cast `/Game/Blueprints/Turret/BP_Turret` PossessedPawn
          (:`then`
            (`EnhancedInputSubsystemInterface.AddMappingContext` _returnvalue "/Game/Input/Turret/IM_Turret.IM_Turret" 0 (struct)))
          (:`CastFailed`
            (cast `/Game/Blueprints/Ghost/BP_SpectatorPawn` PossessedPawn
              (:`then`
                (`EnhancedInputSubsystemInterface.AddMappingContext` _returnvalue "/Game/Input/Spectator/IMC_Spectator.IMC_Spectator" 0 (struct)))
              (:`CastFailed`
                (cast `/Game/Blueprints/Ghost/BP_Ghost` PossessedPawn)
                (`EnhancedInputSubsystemInterface.AddMappingContext` _returnvalue "/Game/Input/Ghost/IMC_Ghost.IMC_Ghost" 0 (struct))))))))))

(event `self.ReceiveUnPossess`
  (params (UnpossessedPawn :type "Pawn Object Reference"))
  (bind _returnvalue (pcsubsystem `EnhancedInputLocalPlayerSubsystem` self))
  ;[1 0.03429 0] Unpossessed Pawn
  ;[0.03737 0.07216 0.151 0.769] Setup input context for possessed pawn
  (cast `/Game/Blueprints/Turret/BP_Turret` UnpossessedPawn
    (:`then`
      (`EnhancedInputSubsystemInterface.RemoveMappingContext` _returnvalue "/Game/Input/Turret/IM_Turret.IM_Turret" (struct)))
    (:`CastFailed`
      (cast `/Game/Blueprints/Ghost/BP_SpectatorPawn` UnpossessedPawn
        (:`then`
          (`EnhancedInputSubsystemInterface.RemoveMappingContext` _returnvalue "/Game/Input/Spectator/IMC_Spectator.IMC_Spectator" (struct)))
        (:`CastFailed`
          (cast `/Game/Blueprints/Ghost/BP_Ghost` UnpossessedPawn)
          (`EnhancedInputSubsystemInterface.RemoveMappingContext` _returnvalue "/Game/Input/Ghost/IMC_Ghost.IMC_Ghost" (struct)))))))

(fn `UserConstructionScript`)