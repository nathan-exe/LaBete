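; PC_Gyroscope turns an Arduino gyroscope gun controller, read over a fixed serial port, into aim and button input.
; BeginPlay opens the port, and a delayed Tick reads its bytes, scanning back to the last 255 marker to locate the newest packet.
; Three packet floats become a camera-relative, interpolated TurretRotation and a PointerDirection vector.
; A bitmask byte drives press and release events on state changes, though Button0's release fires the AnyButton event.
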(event `self.ReceiveEndPlay`
  (params (EndPlayReason :type "EEndPlayReason Enum" :default "Destroyed"))
  (bind _arduinoport (`self.ArduinoPort`))
  ;[1 0.5088 0.467] Close Port
  (`/Engine/EditorBlueprintResources/StandardMacros.IsValid` _arduinoport
    (:`Is Valid`
      (`SerialCom.Close` _arduinoport))))

(event `self.ReceiveBeginPlay`
  (bind _arduinoport (`self.ArduinoPort`))
  ;[1 0.006291 0] Begin Play
  (if true
    (`|ExecutionSequence`
      (:`then_0`
        ;[0.7142 1 0.4643] find serial port
        (bind (_bopened _returnvalue) (`SerialCom.OpenComPort` 3 115200 :!label _label))
        (if _bopened
          (`KismetSystemLibrary.PrintString` (`KismetSystemLibrary.GetDisplayName` _returnvalue) true true (struct :`R` 0.772904 :`G` 1.0 :`A` 1.0) 20.0)
          (bind _output_get (set `self.ArduinoPort` _returnvalue))
          (`SerialCom.Flush` _output_get)
          (bind _returnvalue_2 (`KismetStringLibrary.Concat_StrStr` "serial port opening success : " (`KismetStringLibrary.Conv_BoolToString` _bopened)))
          (`KismetSystemLibrary.PrintString` _returnvalue_2 true true (struct :`R` 0.104774 :`G` 1.0 :`A` 1.0))
          (for _ (`|MakeArray` 300 600 750 1200 2400 9600 19200 31250 38400 57600 74880 115200 230400) :!via `Break`
            (goto _label))
          (else
            (`KismetSystemLibrary.PrintString` _returnvalue_2 true true (struct :`R` 1.0 :`G` 0.099982 :`A` 1.0) 1.0))))
      (:`then_1`
        ;[0.3284 1 0.3075] Print port info
        (`/Engine/EditorBlueprintResources/StandardMacros.IsValid` _arduinoport
          (:`Is Valid`
            (`KismetSystemLibrary.PrintString` (`KismetStringLibrary.Concat_StrStr` "Found Port with id : " (`KismetStringLibrary.Conv_IntToString` (`SerialCom.GetPort` _arduinoport)) " and baud rate : " (`KismetStringLibrary.Conv_IntToString` (`SerialCom.GetBaud` _arduinoport))) true true (struct :`G` 1.0 :`B` 0.069727 :`A` 1.0) 10.0))
          (:`Is Not Valid`
            (`KismetSystemLibrary.PrintString` "Couldn't open any port !!!" true true (struct :`R` 1.0 :`B` 0.05106 :`A` 1.0) 10.0)))))))

(event `self.ReceivePossess`
  (params (PossessedPawn :type "Pawn Object Reference")))

(event `self.ReceiveTick`
  (params (DeltaSeconds :type "Float (single-precision)"))
  (bind _returnvalue (`KismetMathLibrary.Conv_ByteToInt64` 4))
  (bind _returnvalue_2 (`KismetMathLibrary.Conv_ByteToInt64` 1))
  (bind _returnvalue_3 (`KismetMathLibrary.Conv_ByteToInt64` 2))
  (bind _arduinoport (`self.ArduinoPort`))
  ;[1 0.006291 0] Tick
  (`KismetSystemLibrary.Delay` 0.2)
  (`/Engine/EditorBlueprintResources/StandardMacros.IsValid` _arduinoport
    (:`Is Valid`
      (if (`SerialCom.IsOpened` _arduinoport)
        ;[0.6735 0.1441 0.6906] Read Bytes in serial port
        (bind _returnvalue_4 (`SerialCom.ReadBytes` (`self.ArduinoPort`) 10000))
        (bind _returnvalue_5 (`KismetArrayLibrary.Array_Length` _returnvalue_4))
        (if (> _returnvalue_5 0)
          (bind _offset (`self.GetOffsetToLastReadableByte` _returnvalue_4))
          (`|ExecutionSequence`
            (:`then_0`
              (bind _returnvalue_6 (- _returnvalue_5 _offset))
              (bind _returnvalue_7 (`KismetMathLibrary.RInterpTo` (`self.TurretRotation`) (`KismetMathLibrary.ComposeRotators` (`KismetMathLibrary.MakeRotator` (`self.ReadFloatFromByteArray` (- _returnvalue_6 13) _returnvalue_4) (`self.ReadFloatFromByteArray` (- _returnvalue_6 9) _returnvalue_4) (+ (`self.ReadFloatFromByteArray` (- _returnvalue_6 5) _returnvalue_4) 90.0)) (`KismetMathLibrary.NegateRotator` (`PlayerCameraManager.GetCameraRotation` (`GameplayStatics.GetPlayerCameraManager` 0)))) DeltaSeconds 100.0))
              ;[0.4062 0.6251 1] rotation
              (set `self.TurretRotation` _returnvalue_7)
              (set `self.PointerDirection` (* (`KismetMathLibrary.GetRightVector` _returnvalue_7) 1.0)))
            (:`then_1`
              (`|ExecutionSequence`
                (:`then_0`
                  ;[1 0.2586 0.3084] Button Events
                  (`|ExecutionSequence`
                    (:`then_0`
                      (bind _output (`|GetArrayItem` _returnvalue_4 (- _returnvalue_6 1)))
                      (bind _returnvalue_8 (== (`KismetMathLibrary.And_Int64Int64` (`KismetMathLibrary.Conv_ByteToInt64` _output) _returnvalue_2) _returnvalue_2))
                      (if (!= _returnvalue_8 (`self.AnyButton`))
                        (if (`self.AnyButton`)
                          (`self.OnAnyButtonReleased`)
                          (else
                            (`self.OnAnyButtonPressed`)))))
                    (:`then_1`
                      (set `self.AnyButton` _returnvalue_8))))
                (:`then_1`
                  (`|ExecutionSequence`
                    (:`then_0`
                      (bind _returnvalue_9 (== (`KismetMathLibrary.And_Int64Int64` (`KismetMathLibrary.Conv_ByteToInt64` _output) _returnvalue_3) _returnvalue_3))
                      (if (!= _returnvalue_9 (`self.Button_0`))
                        (if (`self.Button_0`)
                          (`self.OnAnyButtonReleased`)
                          (else
                            (`self.OnButton0Pressed`)))))
                    (:`then_1`
                      (set `self.Button_0` _returnvalue_9))))
                (:`then_2`
                  (`|ExecutionSequence`
                    (:`then_0`
                      (bind _returnvalue_10 (== (`KismetMathLibrary.And_Int64Int64` (`KismetMathLibrary.Conv_ByteToInt64` _output) _returnvalue) _returnvalue))
                      (if (!= _returnvalue_10 (`self.Button_1`))
                        (if (`self.Button_1`)
                          (`self.OnButton1Released`)
                          (else
                            (`self.OnButton1Pressed`)))))
                    (:`then_1`
                      (set `self.Button_1` _returnvalue_10)))))))
          (else
            (`KismetSystemLibrary.PrintString` "No bytes in Serial Port !" true true (struct :`R` 1.0 :`B` 0.068793 :`A` 1.0) 0.2)))
        (else
          (`KismetSystemLibrary.PrintString` "No Serial Port !!" true true (struct :`R` 1.0 :`G` 0.018015 :`A` 1.0) 10.0 :!label _label_2))))
    (:`Is Not Valid`
      (goto _label_2))))

(fn `GetOffsetToLastReadableByte`
  (params (array :type "Array of Byte (by ref)"))
  (returns (offset :type Integer))
  (locals (OffsetValue :type Integer))
  (bind _returnvalue (- (`KismetArrayLibrary.Array_Length` array) (`local.OffsetValue`)))
  (while (and (!= (`|GetArrayItem` array _returnvalue) 255) (> _returnvalue 0))
    (`/Engine/EditorBlueprintResources/StandardMacros.IncrementInt` (`local.OffsetValue`)))
  (return (`local.OffsetValue`)))

(fn `UserConstructionScript`)