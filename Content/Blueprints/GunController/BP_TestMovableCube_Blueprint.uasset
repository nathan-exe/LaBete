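; Test cube actor that mirrors an Arduino controller's orientation and button state over a serial COM port, with on-screen debug prints.
; BeginPlay opens the port and EndPlay closes it.
; Each Tick reads the buffered bytes, scans back to the last 255 marker and takes three floats and a button bitmask before it.
; The floats drive an interpolated actor rotation, with pitch and yaw negated, and the lowest bit enlarges the cube.
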(event `self.ReceiveEndPlay`
  (params (EndPlayReason :type "EEndPlayReason Enum" :default "Destroyed"))
  (bind _arduinoport (`self.ArduinoPort`))
  ;[1 0.5088 0.467] Close Port
  (`/Engine/EditorBlueprintResources/StandardMacros.IsValid` _arduinoport
    (:`Is Valid`
      (`SerialCom.Close` _arduinoport))))

(event `self.ReceiveBeginPlay`
  (bind _arduinoport (`self.ArduinoPort`))
  (`|ExecutionSequence`
    (:`then_0`
      ;[0.7142 1 0.4643] find serial port
      (bind (_bopened _returnvalue) (`SerialCom.OpenComPort` 3 115200))
      (if _bopened
        (`KismetSystemLibrary.PrintString` (`KismetSystemLibrary.GetDisplayName` _returnvalue) true true (struct :`R` 0.772904 :`G` 1.0 :`A` 1.0) 20.0)
        (set `self.ArduinoPort` _returnvalue)
        (bind _returnvalue_2 (`KismetStringLibrary.Concat_StrStr` "serial port opening success : " (`KismetStringLibrary.Conv_BoolToString` _bopened)))
        (`KismetSystemLibrary.PrintString` _returnvalue_2 true true (struct :`R` 0.104774 :`G` 1.0 :`A` 1.0))
        (else
          (`KismetSystemLibrary.PrintString` _returnvalue_2 true true (struct :`R` 1.0 :`G` 0.099982 :`A` 1.0) 1.0))))
    (:`then_1`
      ;[0.3284 1 0.3075] Print port info
      (`/Engine/EditorBlueprintResources/StandardMacros.IsValid` _arduinoport
        (:`Is Valid`
          (`KismetSystemLibrary.PrintString` (`KismetStringLibrary.Concat_StrStr` "Found Port with id : " (`KismetStringLibrary.Conv_IntToString` (`SerialCom.GetPort` _arduinoport)) " and baud rate : " (`KismetStringLibrary.Conv_IntToString` (`SerialCom.GetBaud` _arduinoport))) true true (struct :`G` 1.0 :`B` 0.069727 :`A` 1.0) 10.0))
        (:`Is Not Valid`
          (`KismetSystemLibrary.PrintString` "Couldn't open any port !!!" true true (struct :`R` 1.0 :`B` 0.05106 :`A` 1.0) 10.0))))))

(event `self.ReceiveTick`
  (params (DeltaSeconds :type "Float (single-precision)"))
  (bind _returnvalue (`KismetMathLibrary.Conv_ByteToInt64` 1))
  (bind _arduinoport (`self.ArduinoPort`))
  (`|ExecutionSequence`
    (:`then_0`
      (`/Engine/EditorBlueprintResources/StandardMacros.IsValid` _arduinoport
        (:`Is Valid`
          (if (`SerialCom.IsOpened` _arduinoport)
            (bind _returnvalue_2 (`SerialCom.ReadBytes` (`self.ArduinoPort`) 10000))
            (bind _offset (`self.GetOffsetToLastReadableByte` _returnvalue_2))
            (bind _returnvalue_3 (- (`KismetArrayLibrary.Array_Length` _returnvalue_2) _offset))
            (bind _returnvalue_4 (`KismetMathLibrary.MakeRotator` (`self.ReadFloatFromByteArray` (- _returnvalue_3 13) _returnvalue_2) (* (`self.ReadFloatFromByteArray` (- _returnvalue_3 9) _returnvalue_2) -1.0) (* (`self.ReadFloatFromByteArray` (- _returnvalue_3 5) _returnvalue_2) -1.0)))
            ;[0.4062 0.6251 1] rotation
            (`KismetSystemLibrary.PrintString` (`KismetStringLibrary.Conv_RotatorToString` _returnvalue_4))
            (`self.K2_SetActorRotation` (`KismetMathLibrary.RInterpTo` (`self.K2_GetActorRotation`) _returnvalue_4 DeltaSeconds 10.0))
            (else
              (`KismetSystemLibrary.PrintString` "No Serial Port !!" true true (struct :`R` 1.0 :`G` 0.018015 :`A` 1.0) 10.0)
              (`self.K2_DestroyActor`))))))
    (:`then_1`
      (bind _output (`|GetArrayItem` _returnvalue_2 (- _returnvalue_3 1)))
      (`KismetSystemLibrary.PrintString` (`KismetStringLibrary.Conv_ByteToString` _output) true true (struct :`R` 1.0 :`G` 0.128458 :`A` 1.0))
      (if (== (`KismetMathLibrary.And_Int64Int64` (`KismetMathLibrary.Conv_ByteToInt64` _output) _returnvalue) _returnvalue)
        (`self.SetActorScale3D` (1.2 1.2 1.2))
        (else
          (`self.SetActorScale3D` (1.0 1.0 1.0)))))))

(fn `GetOffsetToLastReadableByte`
  (params (array :type "Array of Byte"))
  (returns (offset :type Integer))
  (locals (offsetValue :type Integer))
  (bind _returnvalue (- (`KismetArrayLibrary.Array_Length` array) (`local.offsetValue`)))
  (while (and (!= (`|GetArrayItem` array _returnvalue) 255) (> _returnvalue 0))
    (`/Engine/EditorBlueprintResources/StandardMacros.IncrementInt` (`local.offsetValue`)))
  (return (`local.offsetValue`)))

(fn `UserConstructionScript`)