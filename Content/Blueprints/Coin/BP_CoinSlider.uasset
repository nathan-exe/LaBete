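; BP_CoinSlider is a progress slider that shows the coin count reported by BP_CoinManager.
; Count updates set a clamped target, which a DoOnce-guarded, tick-delayed while loop eases toward with FInterpTo, then snaps to.
; Each step updates the fill's dynamic material and moves the knob between Start and End.
; It also writes SCoin's world location back to the manager as CoinSliderTip.
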(event `self.ReceiveBeginPlay`
  ;[1 0.08141 0.05157] BeginPlay
  (`|ExecutionSequence`
    (:`then_0`
      (bind _returnvalue (`GameplayStatics.GetActorOfClass` "/Game/Blueprints/Coin/BP_CoinManager.BP_CoinManager_C"))
      (bind _output_get (set `self.coinManager` _returnvalue))
      (add `/Game/Blueprints/Coin/BP_CoinManager.OnCoinCountUpdated` _output_get (delegate `On Coin Count Changed`)))
    (:`then_1`
      ;[1 0.3875 0.2067] init dynamic material
      (`/Engine/EditorBlueprintResources/StandardMacros.IsValid` (`self.sliderFillMaterial`)
        (:`Is Not Valid`
          (bind _returnvalue_2 (`PrimitiveComponent.CreateDynamicMaterialInstance` (`self.fillMesh`) 0 null "None"))
          (set `self.sliderFillMaterial` _returnvalue_2)
          (`self.UpdateVisuals`))))))

(event `On Coin Count Changed`
  (params (`new amount` :type Integer) (`max possible amount` :type Integer) (`normalized amount` :type "Float (double-precision)"))
  (`self.SetValue` (/ (+ (`KismetMathLibrary.Conv_IntToDouble` `new amount`) 0.5) (`KismetMathLibrary.Conv_IntToDouble` `max possible amount`))))

(event `SetValue`
  (params (value :type "Float (double-precision)"))
  ;[1 0.02535 0] Set Value
  (set `self.sliderTargetValue` (`KismetMathLibrary.FClamp` value))
  (`/Engine/EditorBlueprintResources/StandardMacros.DoOnce` false :!label _label
    (:`Completed`
      (`/Game/Blueprints/BlueprintLibraries/FlowControlLibrary.WhileLoopWithTickDelay` (not (`KismetMathLibrary.NearlyEqual_FloatFloat` (`self.sliderValue`) (`self.sliderTargetValue`) 0.0001)) self
        (:`loop body`
          ;[1 0.2806 0.1808] Lerp toward target value
          (set `self.sliderValue` (`KismetMathLibrary.FInterpTo` (`self.sliderValue`) (`self.sliderTargetValue`) (`GameplayStatics.GetWorldDeltaSeconds`) 3.0)))
        (:`Finished`
          (`|ExecutionSequence`
            (:`then_0`
              (set `self.sliderValue` (`self.sliderTargetValue`)))
            (:`then_1`
              (goto _label :!via `Reset`)))))
      (`self.UpdateVisuals`))))

(event `UpdateVisuals`
  (bind _returnvalue (`KismetMathLibrary.MapRangeClamped` (`self.sliderValue`) 0.0 1.0 0.05 1.0))
  ;[1 0 0] Update Visuals
  (`|ExecutionSequence`
    (:`then_0`
      ;[0.4158 0.6112 1] Update material
      (`/Engine/EditorBlueprintResources/StandardMacros.IsValid` (`self.sliderFillMaterial`)
        (:`Is Valid`
          (`MaterialInstanceDynamic.SetScalarParameterValue` (`self.sliderFillMaterial`) "sliderValue" _returnvalue))))
    (:`then_1`
      ;[0.3146 0.5071 1] Update knob position
      (`SceneComponent.K2_SetWorldLocation` (`self.knob`) (`KismetMathLibrary.VLerp` (`SceneComponent.K2_GetComponentLocation` (`self.Start`)) (`SceneComponent.K2_GetComponentLocation` (`self.End`)) _returnvalue) false false)
      (set `/Game/Blueprints/Coin/BP_CoinManager.CoinSliderTip` (`SceneComponent.K2_GetComponentLocation` (`self.S_Coin`)) (`self.coinManager`)))))

(fn `UserConstructionScript`)