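; BP_CoinManager is a manager actor that creates the coin HUD widget on BeginPlay and spawns coins around the map.
; A Delay in Tick paces SpawnCoin to about every five seconds, placing BP_Coin randomly within MinPos/MaxPos XY bounds while CoinInMap is at most 10.
; CheckObjectifs resets the coin tally when it equals the objective and prints a placeholder message for a future power spawn.
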(event `self.ReceiveBeginPlay`
  (bind _returnvalue (`|CreateWidget` "/Game/Blueprints/Coin/CoinWidget.CoinWidget_C"))
  (`UserWidget.AddToViewport` _returnvalue 0))

(event `self.ReceiveTick`
  (params (DeltaSeconds :type "Float (single-precision)"))
  (`KismetSystemLibrary.Delay` 5.0)
  (`self.SpawnCoin`))

(event `SpawnCoin`
  (bind (_minpos_x _minpos_y) (`KismetMathLibrary.BreakVector` (`self.MinPos`)))
  (bind (_maxpos_x _maxpos_y) (`KismetMathLibrary.BreakVector` (`self.MaxPos`)))
  (if (<= (`self.CoinInMap`) 10)
    (`|SpawnActorFromClass` "/Game/Blueprints/Coin/BP_Coin.BP_Coin_C" (`KismetMathLibrary.Conv_VectorToTransform` (`KismetMathLibrary.MakeVector` (`KismetMathLibrary.RandomFloatInRange` _minpos_x _maxpos_x) (`KismetMathLibrary.RandomFloatInRange` _minpos_y _maxpos_y) 25.0)) "Undefined" "MultiplyWithRoot" null null)
    (set `self.CoinInMap` (+ (`self.CoinInMap`) 1))))

(event `CheckObjectifs`
  (if (== (`self.actualCoinsAmount`) (`self.CoinsObjectifs`))
    (set `self.actualCoinsAmount` 0)
    (`KismetSystemLibrary.PrintString` "Appeller spawn de pouvoir")))

(fn `UserConstructionScript`)