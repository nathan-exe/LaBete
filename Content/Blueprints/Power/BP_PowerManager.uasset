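; BP_PowerManager spawns random power actors at random reachable points in the level.
; The SpawnPower event calls PowerSpawn for one actor; the function can loop over any requested amount.
; Each iteration picks a navigable point within a huge radius of the world origin and spawns a random PowerList class there, printing debug text for success, failure and loop end.
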(event `self.ReceiveBeginPlay`)

(event `SpawnPower`
  (`self.Power Spawn` 1))

(fn `Power Spawn`
  (params (AmountToSpawn :type Integer))
  (for _ (range 1 (+ AmountToSpawn 1))
    (bind (_randomlocation _returnvalue) (`NavigationSystemV1.K2_GetRandomLocationInNavigableRadius` (`KismetMathLibrary.Vector_Zero`) 1000000.0 null null))
    (if (== _returnvalue true)
      (`|SpawnActorFromClass` (`KismetArrayLibrary.Array_Random` (`self.PowerList`)) (`KismetMathLibrary.MakeTransform` _randomlocation) "Undefined" "MultiplyWithRoot" null null)
      (`KismetSystemLibrary.PrintString` "PowerSpawed")
      (else
        (`KismetSystemLibrary.PrintString` "NoPlaceToSpawn" true true (struct :`R` 1.0 :`G` 0.015783 :`A` 1.0)))))
  (`KismetSystemLibrary.PrintString` "LoopSpawnPowerEnd"))

(fn `UserConstructionScript`)