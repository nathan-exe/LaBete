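; Power-up pickup that a BP_Ghost without an active power collects on overlap, passing it the sprite color before the pickup destroys itself.
; Activate is an empty hook, apparently for child powers, alongside ready-made events for speed boost, invincibility, reviving dead ghosts and blocking the shooter.
; Speed and shield timing run on the ghost, revives use the GameStateManager's ghost manager, and shot blocking uses a local Delay.
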(event `self.ReceiveBeginPlay`
  (bind _returnvalue (`GameplayStatics.GetActorOfClass` "/Game/Blueprints/Shooter/BP_Shooter.BP_Shooter_C"))
  (set `self.ShooterRef` _returnvalue)
  (bind _returnvalue_2 (`GameplayStatics.GetActorOfClass` "/Game/Blueprints/Game/BP_GameStateManager.BP_GameStateManager_C"))
  (set `self.GameStateRef` _returnvalue_2))

(event `self.ReceiveActorBeginOverlap`
  (params (OtherActor :type "Actor Object Reference"))
  (bind _currentghostref (`self.CurrentGhostRef`))
  (bind _asbp_ghost (cast `/Game/Blueprints/Ghost/BP_Ghost` OtherActor))
  (set `self.CurrentGhostRef` _asbp_ghost)
  (if (not (`/Game/Blueprints/Ghost/BP_Ghost.HavePowerEnabled` (`self.CurrentGhostRef`)))
    (set `/Game/Blueprints/Ghost/BP_Ghost.PowerColor` (`PaperSpriteComponent.SpriteColor` (`self.PaperSprite`)) _currentghostref)
    (`/Game/Blueprints/Ghost/BP_Ghost.SetActivePower` _currentghostref true)
    (`self.Activate`)
    (`self.K2_DestroyActor`)))

(event `IncreaseSpeed`
  (params (SpeedFactor :type "Float (double-precision)"))
  (bind _currentghostref (`self.CurrentGhostRef`))
  (set `/Game/Blueprints/Ghost/BP_Ghost.GhostSpeed` (* (`/Game/Blueprints/Ghost/BP_Ghost.GhostSpeed` (`self.CurrentGhostRef`)) SpeedFactor) _currentghostref)
  (`/Game/Blueprints/Ghost/BP_Ghost.SpeedRoutine` _currentghostref (`self.ActivationTimeAmount`) SpeedFactor))

(event `GiveInvicibility`
  (bind _currentghostref (`self.CurrentGhostRef`))
  (`/Game/Blueprints/Ghost/BP_Ghost.EnableInvinciblity` _currentghostref)
  (set `/Game/Blueprints/Ghost/BP_Ghost.InviciblePowerEnable` true _currentghostref)
  (`/Game/Blueprints/Ghost/BP_Ghost.ShieldRoutine` _currentghostref (`self.ActivationTimeAmount`)))

(event `ReviveAllDeathGhost`
  (bind _deathghosts (`/Game/Blueprints/Ghost/BP_GhostManager.GetAllDeadGhost` (`/Game/Blueprints/Game/BP_GameStateManager.GhostManagerRef` (`self.GameStateRef`))))
  (for _array_element _deathghosts
    (`/Game/Blueprints/Ghost/BP_Ghost.RespawnGhost` _array_element)
    (`/Game/Blueprints/Ghost/BP_Ghost.SetActivePower` (`self.CurrentGhostRef`) false)))

(event `ReviveRandomDeathGhost`
  (bind _deathghost (`/Game/Blueprints/Ghost/BP_GhostManager.GetRandomDeathGhost` (`/Game/Blueprints/Game/BP_GameStateManager.GhostManagerRef` (`self.GameStateRef`))))
  (`/Game/Blueprints/Ghost/BP_Ghost.RespawnGhost` _deathghost)
  (`/Game/Blueprints/Ghost/BP_Ghost.SetActivePower` (`self.CurrentGhostRef`) false))

(event `BlockShoot`
  (set `/Game/Blueprints/Shooter/BP_Shooter.CanShoot` false (`self.ShooterRef`))
  (`KismetSystemLibrary.PrintString` "ShootBlockStart")
  (`KismetSystemLibrary.Delay` (`self.ActivationTimeAmount`))
  (set `/Game/Blueprints/Shooter/BP_Shooter.CanShoot` true (`self.ShooterRef`))
  (`KismetSystemLibrary.PrintString` "ShootBlockEnd" true true (struct :`R` 1.0 :`B` 0.148843 :`A` 1.0)))

(event `PlaySound`
  (`KismetSystemLibrary.PrintString` "SoundPlay"))

(event `PlayVFX`
  (`KismetSystemLibrary.PrintString` "VFXPlay")
  ;[1 1 1] Set color of ghost to power color
  (`PaperSpriteComponent.SetSpriteColor` (`/Game/Blueprints/Ghost/BP_Ghost.PaperSprite` (`self.CurrentGhostRef`)) (`PaperSpriteComponent.SpriteColor` (`self.PaperSprite`))))

(fn `Activate`)

(fn `UserConstructionScript`)