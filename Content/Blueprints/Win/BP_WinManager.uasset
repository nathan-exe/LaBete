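; BP_WinManager handles the two match outcomes, a Ghost win or a Shooter (Hunter) win.
; It caches GameMode_Main on BeginPlay for use by both win events.
; Each event creates a W_EndPanel widget, sets that side's win text through EditTimer, and calls EndGame on the game mode with true for Ghost, false for Shooter.
; The Shooter path also prints debug strings; neither event's caller is in this graph.
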(event `self.ReceiveBeginPlay`
  (bind _asgame_mode_main (cast `/Game/Blueprints/GameMode/GameMode_Main` (`GameplayStatics.GetGameMode`)))
  (set `self.GameMode` _asgame_mode_main))

(event `GhostWin`
  (bind _returnvalue (`|CreateWidget` "/Game/Blueprints/Win/W_EndPanel.W_EndPanel_C"))
  (`UserWidget.AddToViewport` _returnvalue 0)
  (`/Game/Blueprints/Win/W_EndPanel.EditTimer` _returnvalue (`self.GhostWinText`))
  (`/Game/Blueprints/GameMode/GameMode_Main.EndGame` (`self.GameMode`) true))

(event `ShooterWin`
  (`KismetSystemLibrary.PrintString` "shooter win" true true (struct :`R` 1.0 :`G` 0.007827 :`A` 1.0) 10.0)
  (bind _returnvalue (`|CreateWidget` "/Game/Blueprints/Win/W_EndPanel.W_EndPanel_C"))
  (`UserWidget.AddToViewport` _returnvalue 0)
  (`/Game/Blueprints/Win/W_EndPanel.EditTimer` _returnvalue (`self.HunterWinText`))
  (`KismetSystemLibrary.PrintString` "AHHHHHHH")
  (`/Game/Blueprints/GameMode/GameMode_Main.EndGame` (`self.GameMode`) false))

(fn `UserConstructionScript`)