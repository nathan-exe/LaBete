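; BP_Canard is a duck Blueprint that switches between walking, running and swimming states, shown only as French debug messages.
; Its Sphere overlap event prints the other actor's display name and matches it against the Ground, Air and Water trigger boxes to set StateID.
; Tick prints the current state's message every frame, with the Air trigger mapped to running.
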(event `self.ReceiveTick`
  (params (DeltaSeconds :type "Float (single-precision)"))
  (switch `int` (`self.StateID`)
    (:`0`
      (`KismetSystemLibrary.PrintString` "Je marche"))
    (:`1`
      (`KismetSystemLibrary.PrintString` "Je cours"))
    (:`2`
      (`KismetSystemLibrary.PrintString` "Je nage"))))

(event `self.Sphere.OnComponentBeginOverlap`
  (params (OverlappedComponent :type "PrimitiveComponent Object Reference") (OtherActor :type "Actor Object Reference") (OtherComp :type "PrimitiveComponent Object Reference") (OtherBodyIndex :type Integer) (bFromSweep :type Boolean) (SweepResult :type "HitResult Structure (by ref)"))
  (bind _returnvalue (`KismetSystemLibrary.GetDisplayName` OtherActor))
  (`KismetSystemLibrary.PrintString` _returnvalue)
  (switch `string` _returnvalue
    (:`TriggerBox_Ground`
      (set `self.StateID` 0))
    (:`TriggerBox_Air`
      (set `self.StateID` 1))
    (:`TriggerBox_Water`
      (set `self.StateID` 2))))

(fn `UserConstructionScript`)