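; Match countdown manager that runs the round timer and calls GhostWin on BP_WinManager when time runs out.
; StartTimer splits the game-settings duration into minutes and seconds and creates the W_Timer widget.
; A recursive one-second Delay loop updates the widget, subtracting only frame delta time per pass rather than a full second.
; Each pass also advances counters that trigger coin and window spawns through GameStateManager's managers at configured intervals.
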(event `self.ReceiveBeginPlay`
  (bind _returnvalue (`GameplayStatics.GetActorOfClass` "/Game/Blueprints/Game/BP_GameStateManager.BP_GameStateManager_C"))
  (set `self.GameStateManagerRef` _returnvalue)
  (set `self.TimeAmount` (`/Game/Blueprints/Game/BP_GameSettingsComponent.GameDuration` (`/Game/Blueprints/Game/BP_GameStateManager.BP_GameSettingsComponent` (`self.GameStateManagerRef`)))))

(event `StartTimer`
  ;[0.717 0.154 1] Start
  (if (>= (`self.TimeAmount`) 60) :!label _label
    (set `self.MinuteLeft` (+ (`self.MinuteLeft`) 1))
    (set `self.TimeAmount` (- (`self.TimeAmount`) 60))
    (goto _label)
    (else
      (set `self.TimeLeft` (`self.TimeAmount`))
      (bind _returnvalue (`|CreateWidget` "/Game/Blueprints/Timer/W_Timer.W_Timer_C"))
      (`UserWidget.AddToViewport` _returnvalue 0)
      (set `self.WidgetRef` _returnvalue)
      (`/Game/Blueprints/Timer/W_Timer.EditTimer` (`self.WidgetRef`) (`self.TimeLeft`) (`self.MinuteLeft`))
      (`self.TimerLoop`))))

(event `TimerLoop`
  ;[1 0.3467 0.1661] TimerLoop
  (`KismetSystemLibrary.Delay` 1.0)
  (`self.CoinLogic`)
  (`self.WindowLogic`)
  (if (<= (`self.TimeLeft`) 0.0)
    (if (<= (`self.MinuteLeft`) 0)
      (`self.EndGame`)
      (else
        (set `self.MinuteLeft` (- (`self.MinuteLeft`) 1))
        (set `self.TimeLeft` (+ (`self.TimeLeft`) 60))
        (bind _output_get (set `self.TimeLeft` (- (`self.TimeLeft`) (`GameplayStatics.GetWorldDeltaSeconds`)) :!label _label_2))
        (`/Game/Blueprints/Timer/W_Timer.EditTimer` (`self.WidgetRef`) _output_get (`self.MinuteLeft`))
        (`self.TimerLoop`)))
    (else
      (goto _label_2))))

(event `EndGame`
  ;[0 1 0.3294] TimerFinish
  (bind _returnvalue (`GameplayStatics.GetActorOfClass` "/Game/Blueprints/Win/BP_WinManager.BP_WinManager_C"))
  (`/Game/Blueprints/Win/BP_WinManager.GhostWin` _returnvalue))

(fn `CoinLogic`
  (bind _result (`/Engine/EditorBlueprintResources/StandardMacros.IncrementInt` (`self.CoinCount`))
    (:`  `
      (if (>= _result (`/Game/Blueprints/Game/BP_GameSettingsComponent.CoinFrequenceTime` (`/Game/Blueprints/Game/BP_GameStateManager.BP_GameSettingsComponent` (`self.GameStateManagerRef`))))
        (`/Game/Blueprints/Coin/BP_CoinManager.SpawnCoin` (`/Game/Blueprints/Game/BP_GameStateManager.CoinManagerRef` (`self.GameStateManagerRef`)))
        (set `self.CoinCount` 0)))))

(fn `UserConstructionScript`)

(fn `WindowLogic`
  (bind _result (`/Engine/EditorBlueprintResources/StandardMacros.IncrementInt` (`self.WindowCount`))
    (:`  `
      (if (>= _result (`/Game/Blueprints/Game/BP_GameSettingsComponent.WindowFrequenceTime` (`/Game/Blueprints/Game/BP_GameStateManager.BP_GameSettingsComponent` (`self.GameStateManagerRef`))))
        (`/Game/Blueprints/Windows/BP_WindowsManager.SpawnWindow` (`/Game/Blueprints/Game/BP_GameStateManager.WindowsManagerRef` (`self.GameStateManagerRef`)))
        (set `self.WindowCount` 0)))))