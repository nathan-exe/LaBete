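; BP_GhostManager tracks living and dead ghosts and triggers the shooter's win through WinManager when the alive list is empty.
; Update Ghost List gathers every BP_Ghost in the level and adds those with health left to the alive list, which helper functions also edit.
; GetRandomDeathGhost picks from zero-health ghosts collected by GetAllDeadGhost, which appends to DeathGhost without clearing it.
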(fn `AddToAliveList`
  (params (Ghost :type "/Game/Blueprints/Ghost/BP_Ghost Object Reference"))
  (`KismetArrayLibrary.Array_Add` (`self.GhostAliveList`) Ghost))

(fn `Check Current Alive Ghosts`
  (if (`KismetArrayLibrary.Array_IsEmpty` (`self.GhostAliveList`))
    (`/Game/Blueprints/Win/BP_WinManager.ShooterWin` (`self.WinManager`))))

(fn `GetAllDeadGhost`
  (returns (DeathGhosts :type "Array of /Game/Blueprints/Ghost/BP_Ghost Object Reference"))
  (locals (DeathGhost :type "Array of /Game/Blueprints/Ghost/BP_Ghost Object Reference"))
  (for _array_element (`self.GhostList`)
    (if (<= (`/Game/Blueprints/Ghost/BP_Ghost.CurrentHealth` _array_element) 0)
      (`KismetArrayLibrary.Array_Add` (`local.DeathGhost`) _array_element)))
  (return (`local.DeathGhost`)))

(fn `GetRandomDeathGhost`
  (returns (DeathGhost :type "/Game/Blueprints/Ghost/BP_Ghost Object Reference"))
  (bind _deathghosts (`self.GetAllDeadGhost`))
  (return (`KismetArrayLibrary.Array_Random` _deathghosts)))

(fn `RemoveFromAliveList`
  (params (GhostDead :type "/Game/Blueprints/Ghost/BP_Ghost Object Reference"))
  (`KismetArrayLibrary.Array_RemoveItem` (`self.GhostAliveList`) GhostDead))

(fn `Update Ghost List`
  (bind _outactors (`GameplayStatics.GetAllActorsOfClass` "/Game/Blueprints/Ghost/BP_Ghost.BP_Ghost_C"))
  (bind _output_get (set `self.GhostList` _outactors))
  (for _array_element _output_get
    (if (> (`/Game/Blueprints/Ghost/BP_Ghost.CurrentHealth` _array_element) 0)
      (`self.AddToAliveList` _array_element))))

(fn `UserConstructionScript`)