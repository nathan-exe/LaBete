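; Turret component that turns Arduino gyroscope and button input into aiming, shooting and game start/restart.
; Until calibrated, each press records an offset-corrected direction at successive targets, with the angle offset derived from the first.
; It then finds the turret position by marching a plane until rays back-projected from the targets converge, saving it in the GameInstance.
; Each tick it raycasts from that position onto the RaycastPlane and smooths the turret's pointer.
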(event `self.ReceiveBeginPlay`
  (bind _calibrationtargets (`self.CalibrationTargets`))
  ;[1 0 0.01765] BeginPlay
  (`|ExecutionSequence`
    (:`then_0`
      ;[0.4843 0.6668 1] Hide Calibration Targets at start
      (for _array_element _calibrationtargets
        (`Actor.SetActorHiddenInGame` _array_element true))
      (`Actor.SetActorHiddenInGame` (`|GetArrayItem` _calibrationtargets) false))
    (:`then_1`
      (bind _asbp_turret (cast `/Game/Blueprints/Turret/BP_Turret` (`self.GetOwner`)))
      (set `self.turret` _asbp_turret))
    (:`then_2`
      (bind _asbp_game_instance (cast `/Game/Blueprints/Game/BP_GameInstance` (`GameplayStatics.GetGameInstance`)))
      (set `self.GameInstance` _asbp_game_instance)
      (bind _output_get (set `self.Calibrated` (`/Game/Blueprints/Game/BP_GameInstance.calibratedTurret` _asbp_game_instance)))
      (if _output_get
        _))
    (:`then_3`
      (bind _asgame_mode_main (cast `/Game/Blueprints/GameMode/GameMode_Main` (`GameplayStatics.GetGameMode`)))
      (set `self.GameMode` _asgame_mode_main))))

(event `init arduino`
  (bind _arduino (`self.Arduino`))
  ;[1 0 0.01492] init arduino
  (add `/Game/Blueprints/Turret/AC_PhysicalGunControllerInterface.OnAnyButtonPressed` _arduino (delegate `OnShoot`))
  (add `/Game/Blueprints/Turret/AC_PhysicalGunControllerInterface.OnBothButtonReleased` _arduino (delegate `OnAnyButtonPressed_Event`)))

(event `OnAnyButtonPressed_Event`
  (`/Game/Blueprints/Turret/BP_Turret.StopShooting` (`self.turret`)))

(event `OnShoot`
  (bind _calibrationtargets (`self.CalibrationTargets`))
  (bind _gameinstance (`self.GameInstance`))
  (bind _gamemode (`self.GameMode`))
  ;[1 0 0.01765] On Shoot
  (if (`self.Calibrated`)
    (bind _returnvalue (`/Game/Blueprints/GameMode/GameMode_Main.IsInCalibrationPhase` _gamemode))
    (if _returnvalue
      (`/Game/Blueprints/GameMode/GameMode_Main.StartGame` (`self.GameMode`))
      (elif (`/Game/Blueprints/GameMode/GameMode_Main.CanRelaunchGame` _gamemode)
        (`/Game/Blueprints/GameMode/GameMode_Main.RestartGame` (`self.GameMode`))
        (else
          (`/Game/Blueprints/Turret/BP_Turret.Shoot` (`self.turret`)))))
    (else
      ;[0.09543 0.47 1] Calibration
      (if (`KismetArrayLibrary.Array_IsEmpty` (`self.ReferenceDirections`))
        (bind _offset (`self.Compute Angle Offset` (`/Game/Blueprints/Turret/AC_PhysicalGunControllerInterface.PointerDirection` (`self.Arduino`))))
        (set `self.AngleOffset` _offset))
      ;;[0.2465 1 0.9303] Register Reference Direction
      (bind _returnvalue_2 (`KismetArrayLibrary.Array_Add` (`self.ReferenceDirections`) (`self.GetCorrectedPointerDirection`)))
      (`|ExecutionSequence`
        (:`then_0`
          ;;[0.4843 0.6668 1] Enable Next Target
          (`|ExecutionSequence`
            (:`then_0`
              (`Actor.SetActorHiddenInGame` (`|GetArrayItem` _calibrationtargets (`KismetMathLibrary.Clamp` (+ _returnvalue_2 1) 0 (- (`KismetArrayLibrary.Array_Length` _calibrationtargets) 1))) false))
            (:`then_1`
              (`Actor.SetActorHiddenInGame` (`|GetArrayItem` _calibrationtargets _returnvalue_2) true))))
        (:`then_1`
          ;;[0.343 1 0.9701] Calibartion end
          (if (== _returnvalue_2 (- (`KismetArrayLibrary.Array_Length` (`self.CalibrationTargets`)) 1))
            (`KismetSystemLibrary.PrintString` "=== Calibration Phase Over ===" true true (struct :`R` 1.0 :`G` 0.513482 :`A` 1.0) 100.0)
            (bind _turretposition (`self.Find Turret Position`))
            (`KismetSystemLibrary.PrintString` (`KismetStringLibrary.Concat_StrStr` "Turret position : " (`KismetStringLibrary.Conv_VectorToString` _turretposition)) true true (struct :`R` 1.0 :`G` 0.736495 :`B` 0.399075 :`A` 1.0) 100.0)
            (set `/Game/Blueprints/Game/BP_GameInstance.TurretPosition` _turretposition _gameinstance)
            (set `/Game/Blueprints/Game/BP_GameInstance.calibratedTurret` true _gameinstance)
            (set `self.Calibrated` true)
            (`KismetSystemLibrary.DelayUntilNextTick`)
            (`/Game/Blueprints/GameMode/GameMode_Main.StartGame` (`self.GameMode`))))))))

(event `self.ReceiveTick`
  (params (DeltaSeconds :type "Float (single-precision)"))
  (bind _raycastplane (`self.RaycastPlane`))
  ;[1 0 0.01765] Tick
  (if (`/Game/Blueprints/Game/BP_GameInstance.calibratedTurret` (`self.GameInstance`))
    (`|ExecutionSequence`
      (:`then_0`
        ;[0.1985 0.8801 1] Compute pointer position
        (bind _hitpoint (`self.Raycast Against Plane` (`Actor.GetActorUpVector` _raycastplane) (`Actor.K2_GetActorLocation` _raycastplane) 0.0 (`/Game/Blueprints/Game/BP_GameInstance.TurretPosition` (`self.GameInstance`)) (`self.GetCorrectedPointerDirection`)))
        (bind _output_get (set `self.pointer` (`KismetMathLibrary.VInterpTo` (stale _output_get) _hitpoint DeltaSeconds 7.0)))
        (`|ExecutionSequence`
          (:`then_0`
            (`/Game/Blueprints/Turret/BP_Turret.SetPointerPosition` (`self.turret`) _output_get))
          (:`then_1`
            (if (`self.debug`)
              ;[1 0.5644 0.1703] Debug Draw Cursor
              (`KismetSystemLibrary.DrawDebugSphere` _output_get 20.0 12 (struct :`R` 1.0 :`G` 0.00692 :`A` 1.0) 0.0 5.0)
              (`KismetSystemLibrary.DrawDebugLine` (0.0 0.0 0.0) _output_get (struct :`R` 0.41886 :`G` 1.0 :`B` 0.178601 :`A` 1.0) 0.0 5.0)
              (`KismetSystemLibrary.DrawDebugLine` (`Actor.K2_GetActorLocation` (`self.RaycastPlane`)) _output_get (struct :`R` 0.846288 :`G` 1.0 :`B` 0.836953 :`A` 1.0) 0.0 5.0)))))
      (:`then_1`
        (`self.Draw Debug After Calibartion`)))
    (else
      (`self.DrawDebugBeforeCalibration`))))

(event `Draw Debug After Calibartion`
  ;[1 0.9175 0.3312] Debug Draw
  (if (`self.debug`)
    (`|ExecutionSequence`
      (:`then_0`)
      (:`then_1`
        ;;[1 0.3904 0.2705] Turret position
        (`KismetSystemLibrary.DrawDebugSphere` (0.0 0.0 0.0) 100.0 12 (struct :`R` 0.397902 :`G` 1.0 :`B` 0.626033 :`A` 1.0) 0.0 1.0))
      (:`then_2`)
      (:`then_3`
        ;;[1 0.5233 0.4534] Reference Directions
        (for (_array_element _array_index) (`self.ReferenceDirections`) :!label _label
          (bind _returnvalue (`Actor.K2_GetActorLocation` (`|GetArrayItem` (`self.CalibrationTargets`) _array_index)))
          (`KismetSystemLibrary.DrawDebugLine` _returnvalue (+ (* (* _array_element 5000.0) -1.0) _returnvalue) (struct :`R` 1.0 :`G` 0.01685 :`A` 1.0) 0.0 2.0))))))

(event `DrawDebugBeforeCalibration`
  ;[1 0.9175 0.3312] Debug Draw
  (if (`self.debug`)
    (`|ExecutionSequence`
      (:`then_0`)
      (:`then_1`
        (goto _label))
      (:`then_2`
        ;;[1 0.5094 0.4195] Cursor direction
        (`KismetSystemLibrary.DrawDebugLine` (0.0 0.0 0.0) (+ (0.0 0.0 0.0) (* (`self.GetCorrectedPointerDirection`) 200.0)) (struct :`R` 1.0 :`G` 0.947917 :`B` 0.947917 :`A` 1.0) 0.0 6.0)))))

(fn `Compute Angle Offset`
  (params (`ref forward` :type "Vector Structure"))
  (returns (offset :type "Rotator Structure"))
  (locals (bestIndex :type Integer))
  (bind _returnvalue (`KismetMathLibrary.Vector_Down`))
  (bind _array (`|MakeArray` (`KismetMathLibrary.Vector_Up`) (`KismetMathLibrary.Vector_Down`) (`KismetMathLibrary.Vector_Forward`) (`KismetMathLibrary.Vector_Backward`) (`KismetMathLibrary.Vector_Left`) (`KismetMathLibrary.Vector_Right`)))
  (bind _returnvalue_2 (`KismetMathLibrary.Vector_SlerpNormals` (`|GetArrayItem` _array (`local.bestIndex`)) `ref forward` 0.02))
  (bind _returnvalue_3 (`KismetMathLibrary.Quat_Rotator` (`KismetMathLibrary.Quat_FindBetweenNormals` _returnvalue_2 _returnvalue)))
  (`KismetSystemLibrary.PrintString` (`KismetStringLibrary.Conv_VectorToString` `ref forward`) true true (struct :`G` 0.66 :`B` 1.0 :`A` 1.0) 50.0)
  (for (_array_element _array_index) _array
    (if (> (`KismetMathLibrary.Dot_VectorVector` _array_element `ref forward`) (`KismetMathLibrary.Dot_VectorVector` `ref forward` (`|GetArrayItem` _array (`local.bestIndex`))))
      (set `local.bestIndex` _array_index)))
  (`KismetSystemLibrary.PrintString` (`KismetStringLibrary.Concat_StrStr` "input : " (`KismetStringLibrary.Conv_VectorToString` `ref forward`) ", best match :" (`KismetStringLibrary.Conv_VectorToString` _returnvalue_2)) true true (struct :`R` 1.0 :`G` 0.757277 :`B` 0.72737 :`A` 1.0) 50.0)
  (`KismetSystemLibrary.PrintString` (`KismetStringLibrary.Concat_StrStr` "compensation : " (`KismetStringLibrary.Conv_DoubleToString` (.roll _returnvalue_3)) "," (`KismetStringLibrary.Conv_DoubleToString` (.pitch _returnvalue_3)) "," (`KismetStringLibrary.Conv_DoubleToString` (.yaw _returnvalue_3)) "  from : " (`KismetStringLibrary.Conv_VectorToString` _returnvalue_2) " to : " (`KismetStringLibrary.Conv_VectorToString` _returnvalue)) true true (struct :`R` 1.0 :`G` 0.757277 :`B` 0.72737 :`A` 1.0) 50.0)
  (return _returnvalue_3))

(fn `ComputeAverageDistanceBetweenPoints`
  (params (vectors :type "Array of Vector Structure (by ref)"))
  (returns (AveragePoint :type "Vector Structure") (AverageDistanceToAveragePoint :type "Float (double-precision)"))
  (locals (Sum :type "Vector Structure") (DistanceSum :type "Float (double-precision)") (DistanceSumCount :type Integer) (averagePosition :type "Vector Structure"))
  (bind _returnvalue (`KismetArrayLibrary.Array_Length` vectors))
  (for _array_element vectors
    (set `local.Sum` (+ _array_element (`local.Sum`))))
  (bind _output_get (set `local.averagePosition` (/ (`local.Sum`) _returnvalue)))
  (for _array_element_2 vectors
    (set `local.DistanceSum` (+ (`KismetMathLibrary.Vector_Distance` _array_element_2 _output_get) (`local.DistanceSum`))))
  (return _output_get (/ (`local.DistanceSum`) _returnvalue)))

(fn `Find Turret Position`
  (returns (TurretPosition :type "Vector Structure"))
  (locals (AveragePoint :type "Vector Structure") (AllHitPoints :type "Array of Vector Structure") (LastAverageDistance :type "Float (double-precision)" :default 1e+24) (CurrentAverageDistance :type "Float (double-precision)" :default 1e+24) (t :type "Float (double-precision)") (iterations :type Integer) (LastAverageDistance :type "Float (double-precision)"))
  (bind _raycastplane (`self.RaycastPlane`))
  (bind _returnvalue (< (`local.iterations`) 10000))
  ;[1 0.6739 0.5157] While the average distance between the lines is decreasing
  (while (and (<= (`local.CurrentAverageDistance`) (`local.LastAverageDistance`)) _returnvalue)
    (`/Engine/EditorBlueprintResources/StandardMacros.IncrementInt` (`local.iterations`)
      (:`  `
        (bind _returnvalue_2 (+ (stale _output_get) 1.0))
        ;[1 0.5116 0.3568] March along Planes
        (bind _output_get (set `local.t` _returnvalue_2))
        (`KismetSystemLibrary.PrintString` (`KismetStringLibrary.Concat_StrStr` "t : " (`KismetStringLibrary.Conv_DoubleToString` _returnvalue_2)) true true (struct :`R` 0.105076 :`G` 0.406284 :`B` 1.0 :`A` 1.0) 20.0)
        (`KismetArrayLibrary.Array_Clear` (`local.AllHitPoints`))
        (for (_array_element _array_index) (`self.ReferenceDirections`)
          ;[1 0.4488 0.2698] Compute all 5 hit points on plane
          (bind _hitpoint (`self.Raycast Against Plane` (* (`Actor.GetActorUpVector` _raycastplane) -1.0) (`Actor.K2_GetActorLocation` _raycastplane) (* (`local.t`) -1.0) (`Actor.K2_GetActorLocation` (`|GetArrayItem` (`self.CalibrationTargets`) _array_index)) (* _array_element -1.0)))
          (`KismetArrayLibrary.Array_Add` (`local.AllHitPoints`) _hitpoint))
        ;[0.375 0.2843 0.2441] Compute average distance between points on plane
        (bind (_averagepoint _averagedistancetoaveragepoint) (`self.ComputeAverageDistanceBetweenPoints` (`local.AllHitPoints`)))
        (set `local.LastAverageDistance` (`local.CurrentAverageDistance`))
        (set `local.CurrentAverageDistance` _averagedistancetoaveragepoint)
        (set `local.AveragePoint` _averagepoint))))
  (if _returnvalue
    (return (`local.AveragePoint`))
    (else
      (`KismetSystemLibrary.PrintString` "bug de salopard ça a failli exploser !" true true (struct :`R` 1.0 :`B` 0.029284 :`A` 1.0) 100.0))))

(fn `Raycast Against Plane`
  (params (PlaneNormal :type "Vector Structure") (PlaneStartPoint :type "Vector Structure") (PlaneOffsetAlongNormal :type "Float (double-precision)") (RayStart :type "Vector Structure") (RayDirection :type "Vector Structure"))
  (returns (HitPoint :type "Vector Structure"))
  (bind _returnvalue (`KismetMathLibrary.Normal` RayDirection))
  (bind _returnvalue_2 (`KismetMathLibrary.Normal` PlaneNormal))
  (bind _returnvalue_3 (* (/ (`KismetMathLibrary.Dot_VectorVector` _returnvalue_2 (- RayStart (+ PlaneStartPoint (* _returnvalue_2 PlaneOffsetAlongNormal)))) (`KismetMathLibrary.Dot_VectorVector` _returnvalue _returnvalue_2)) -1.0))
  (if (< _returnvalue_3 0.0)
    _
    (else
      _))
  (return (+ RayStart (* _returnvalue_3 _returnvalue))))