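; Actor component that gives mouse control of its owning BP_Turret, which it casts and caches at BeginPlay.
; Either mouse button starts shooting on press and stops on release.
; Mouse2D input, when changed since the last event, is axis-swapped, scaled and accumulated into a cursor position passed to the turret as its pointer.
; Releasing Space also calls StartGame on GameMode_Main.
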(event `self.ReceiveTick`
  (params (DeltaSeconds :type "Float (single-precision)")))

(event `Key|RightMouseButton`
  (params (Key :type "Key Structure"))
  (bind _turret (`self.Turret`))
  (:`Pressed`
    (`/Game/Blueprints/Turret/BP_Turret.Shoot` _turret :!label _label))
  (:`Released`
    (`/Game/Blueprints/Turret/BP_Turret.StopShooting` _turret :!label _label_2)))

(event `Key|LeftMouseButton`
  (params (Key :type "Key Structure"))
  (:`Pressed`
    (goto _label))
  (:`Released`
    (goto _label_2)))

(event `self.ReceiveBeginPlay`
  ;[1 0.01447 0] Begin Play
  (bind _asbp_turret (cast `/Game/Blueprints/Turret/BP_Turret` (`self.GetOwner`)))
  (set `self.Turret` _asbp_turret))

(event `InputVectorAxis|Mouse2D`
  (params (AxisValue :type "Vector Structure"))
  ;[1 0.009182 0] Mouse movement
  (`|ExecutionSequence`
    (:`then_0`
      (`GameUserSettings.GetGameUserSettings`)
      (if (!= AxisValue (`self.OldPosition`) :`ErrorTolerance` 1e-05)
        (bind _output_get (set `self.CursorPosition` (+ (stale _output_get) (`KismetMathLibrary.MakeVector` (.y (* AxisValue 9.0)) (.x (* AxisValue 9.0))))))
        (`/Game/Blueprints/Turret/BP_Turret.SetPointerPosition` (`self.Turret`) _output_get)))
    (:`then_1`
      (set `self.OldPosition` AxisValue))))

(event `Key|SpaceBar`
  (params (Key :type "Key Structure"))
  (:`Released`
    (bind _asgame_mode_main (cast `/Game/Blueprints/GameMode/GameMode_Main` (`GameplayStatics.GetGameMode`)))
    (`/Game/Blueprints/GameMode/GameMode_Main.StartGame` _asgame_mode_main)))