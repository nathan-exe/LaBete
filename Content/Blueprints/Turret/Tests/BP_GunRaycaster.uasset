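; Test turret gun actor that calibrates a four-corner aiming area and locates the aimed point within it.
; Shoot events record corners by projecting the actor's yaw and pitch through tangents onto a fixed X plane.
; Once calibrated, Tick splits the quad along a diagonal, picks the triangle with a dot product, and prints the point's barycentric coordinates.
; Debug draws show the area, diagonal, normal and aim direction; line-trace code is disconnected.
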(event `Shoot`
  ;[1 0.03862 0] On Shoot
  (`KismetSystemLibrary.PrintString` "====== \nSHOOT \n======" true true (struct :`R` 1.0 :`B` 0.058903 :`A` 1.0))
  (if (<= (`KismetArrayLibrary.Array_Length` (`self.Angles`)) 4)
    ;[1 0.6982 0.3257] store the 4 angle points coordinates for reference during the calibration phase
    (`KismetArrayLibrary.Array_Add` (`self.Angles`) (`self.GetRawAimedPoint`))))

(event `self.ReceiveTick`
  (params (DeltaSeconds :type "Float (single-precision)"))
  (bind _returnvalue (`self.K2_GetActorLocation`))
  (bind _returnvalue_2 (`self.K2_GetActorLocation`))
  (bind _point (`self.GetRawAimedPoint`))
  (bind _angles (`self.Angles`))
  (bind _angles_2 (`self.Angles`))
  (bind _angles_3 (`self.Angles`))
  (bind _angles_4 (`self.Angles`))
  (bind _angles_5 (`self.Angles`))
  (bind _angles_6 (`self.Angles`))
  (bind _output (`|GetArrayItem` _angles_5 3))
  (bind _output_2 (`|GetArrayItem` _angles 3))
  (bind _returnvalue_3 (- (`|GetArrayItem` _angles 1) _output_2))
  (bind _returnvalue_4 (> (`KismetArrayLibrary.Array_Length` (`self.Angles`)) 3))
  ;[1 0.021 0] OnTick
  (`|ExecutionSequence`
    (:`then_0`
      ;[1 0.4075 0.2613] After Calibration
      (if (>= (`KismetArrayLibrary.Array_Length` (`self.Angles`)) 4)
        ;[0.1745 0.4796 1] Check in wich triangle the point lies
        (if (> (`KismetMathLibrary.Dot_VectorVector` (- _point _output) (`KismetMathLibrary.MakeVector` (.x (- (`|GetArrayItem` _angles_5 1) _output)) (* (.z (- (`|GetArrayItem` _angles_5 1) _output)) -1.0) (.y (- (`|GetArrayItem` _angles_5 1) _output)))) 0.0)
          (`KismetSystemLibrary.DrawDebugPoint` _point 10.0 (struct :`R` 1.0 :`B` 0.212457 :`A` 1.0))
          (`KismetSystemLibrary.PrintString` (`KismetStringLibrary.Concat_StrStr` "Triangle 2. Barycentric :" (`KismetStringLibrary.Conv_VectorToString` (`self.CartesianToBarycentric` (`KismetMathLibrary.MakeVector2D` (.y _point) (.z _point)) (`KismetMathLibrary.MakeVector2D` (.y (`|GetArrayItem` _angles_6)) (.z (`|GetArrayItem` _angles_6))) (`KismetMathLibrary.MakeVector2D` (.y (`|GetArrayItem` _angles_6 1)) (.z (`|GetArrayItem` _angles_6 1))) (`KismetMathLibrary.MakeVector2D` (.y (`|GetArrayItem` _angles_6 3)) (.z (`|GetArrayItem` _angles_6 3)))))))
          (else
            (`KismetSystemLibrary.DrawDebugPoint` _point 10.0 (struct :`G` 1.0 :`B` 0.871732 :`A` 1.0))
            (`KismetSystemLibrary.PrintString` (`KismetStringLibrary.Concat_StrStr` "Triangle 2. Barycentric :" (`KismetStringLibrary.Conv_VectorToString` (`self.CartesianToBarycentric` (`KismetMathLibrary.MakeVector2D` (.y _point) (.z _point)) (`KismetMathLibrary.MakeVector2D` (.y (`|GetArrayItem` _angles_4 1)) (.z (`|GetArrayItem` _angles_4 1))) (`KismetMathLibrary.MakeVector2D` (.y (`|GetArrayItem` _angles_4 2)) (.z (`|GetArrayItem` _angles_4 2))) (`KismetMathLibrary.MakeVector2D` (.y (`|GetArrayItem` _angles_4 3)) (.z (`|GetArrayItem` _angles_4 3)))))))))))
    (:`then_1`
      (`|ExecutionSequence`
        (:`then_0`
          ;[0.5652 1 0.4755] Debug Draw reference points and area
          (for (_array_element _array_index) _angles_2
            (`KismetSystemLibrary.DrawDebugPoint` _array_element 0.2 (struct :`R` 0.943906 :`G` 0.237762 :`B` 1.0 :`A` 1.0))
            (`KismetSystemLibrary.DrawDebugLine` _array_element (`|GetArrayItem` _angles_2 (mod (+ _array_index 1) (`KismetArrayLibrary.Array_Length` _angles_2))) (struct :`R` 0.947307 :`G` 0.238398 :`B` 1.0 :`A` 1.0) 0.0 1.0)))
        (:`then_1`
          (if _returnvalue_4
            (`KismetSystemLibrary.DrawDebugLine` (`|GetArrayItem` _angles_3 1) (`|GetArrayItem` _angles_3 3) (struct :`R` 0.947307 :`G` 0.238398 :`B` 1.0 :`A` 1.0) 0.0 1.0)))
        (:`then_2`
          (if _returnvalue_4
            (`KismetSystemLibrary.DrawDebugLine` _output_2 (+ (`KismetMathLibrary.MakeVector` (.x _returnvalue_3) (* (.z _returnvalue_3) -1.0) (.y _returnvalue_3)) _output_2) (struct :`G` 1.0 :`B` 0.379239 :`A` 1.0) 0.0 1.0)
            (`KismetSystemLibrary.DrawDebugLine` _output_2 (+ _returnvalue_3 _output_2) (struct :`R` 1.0 :`G` 0.251089 :`B` 0.415672 :`A` 1.0) 0.0 1.0)))))
    (:`then_2`
      ;[0.4836 1 0.6408] Draw debug direction
      (`KismetSystemLibrary.DrawDebugArrow` _returnvalue_2 (+ _returnvalue_2 (* (`self.GetActorForwardVector`) 100.0)) 2.0 (struct :`R` 1.0 :`G` 0.240592 :`B` 0.894745 :`A` 0.723) 0.0 1.0)
      (`KismetSystemLibrary.DrawDebugLine` _returnvalue (+ _returnvalue (* (`self.GetActorForwardVector`) 10000.0)) (struct :`R` 0.874322 :`G` 0.562302 :`B` 0.922917 :`A` 0.409) 0.0 1.0))))

(fn `InvLerpVector`
  (params (From :type "Vector Structure") (To :type "Vector Structure") (Value :type "Vector Structure"))
  (returns (NewParam3 :type "Float (double-precision)"))
  (return (/ (`KismetMathLibrary.Dot_VectorVector` (- To From) (- Value From)) (`KismetMathLibrary.Vector_Distance` From To))))

(fn `UserConstructionScript`)