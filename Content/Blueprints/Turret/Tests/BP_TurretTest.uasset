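; Test turret pawn that calibrates its position from gyroscope pointer input, then draws a debug aim cursor on a reference plane.
; Each button press records the pointer direction for the visible calibration target and reveals the next.
; FindTurretPosition steps an offset plane along the reversed rays until their hit points stop converging, then the turret teleports to that average point.
; Tick applies the controller's turret rotation and draws the debug rays and cursor.
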(event `self.ReceiveBeginPlay`
  (bind _calibrationtargets (`self.CalibrationTargets`))
  ;[1 0 0.01765] BeginPlay
  (`|ExecutionSequence`
    (:`then_0`
      ;[0.4843 0.6668 1] Hide Calibration Targets at start
      (for _array_element _calibrationtargets
        (`self.SetActorHiddenInGame` _array_element true))
      (`self.SetActorHiddenInGame` (`|GetArrayItem` _calibrationtargets) false))))

(event `self.ReceivePossessed`
  (params (NewController :type "Controller Object Reference"))
  ;[1 0 0.01492] Possessed
  (bind _aspc_gyroscope (cast `/Game/Blueprints/Turret/Tests/PC_Gyroscope` (`self.GetController`)))
  (bind _output_get (set `self.GyroscopeController` _aspc_gyroscope))
  (add `/Game/Blueprints/Turret/Tests/PC_Gyroscope.OnAnyButtonPressed` _output_get (delegate `OnShoot`)))

(event `OnShoot`
  (bind _calibrationtargets (`self.CalibrationTargets`))
  (bind _pointerdirection (`/Game/Blueprints/Turret/Tests/PC_Gyroscope.PointerDirection` (`self.GyroscopeController`)))
  ;[1 0 0.01765] On Shoot
  (`KismetSystemLibrary.PrintString` "shoot" true true (struct :`R` 0.644457 :`G` 0.97012 :`B` 1.0 :`A` 1.0) 1.0)
  (if (< (`KismetArrayLibrary.Array_Length` (`self.ReferenceDirections`)) (`KismetArrayLibrary.Array_Length` (`self.CalibrationTargets`)))
    ;[1 0.494 0.06162] Register Reference Direction
    (bind _returnvalue (`KismetArrayLibrary.Array_Add` (`self.ReferenceDirections`) _pointerdirection))
    (`KismetSystemLibrary.PrintString` (`KismetStringLibrary.Conv_VectorToString` _pointerdirection) true true (struct :`R` 0.158962 :`G` 1.0 :`A` 1.0) 500.0)
    (`|ExecutionSequence`
      (:`then_0`
        ;[0.4843 0.6668 1] Enable Next Target
        (`|ExecutionSequence`
          (:`then_0`
            (`self.SetActorHiddenInGame` (`|GetArrayItem` _calibrationtargets (`KismetMathLibrary.Clamp` (+ _returnvalue 1) 0 (- (`KismetArrayLibrary.Array_Length` _calibrationtargets) 1))) false))
          (:`then_1`
            (`self.SetActorHiddenInGame` (`|GetArrayItem` _calibrationtargets _returnvalue) true))))
      (:`then_1`
        ;[0.3195 0.5941 1] Calibartion end
        (if (== _returnvalue (- (`KismetArrayLibrary.Array_Length` (`self.CalibrationTargets`)) 1))
          (`KismetSystemLibrary.PrintString` "=== Calibration Phase Over ===" true true (struct :`R` 1.0 :`G` 0.513482 :`A` 1.0) 100.0)
          (bind _turretposition (`self.FindTurretPosition`))
          (`KismetSystemLibrary.PrintString` (`KismetStringLibrary.Concat_StrStr` "Turret position : " (`KismetStringLibrary.Conv_VectorToString` _turretposition)) true true (struct :`R` 0.819825 :`G` 0.195823 :`B` 1.0 :`A` 1.0) 100.0)
          (`self.K2_SetActorLocation` _turretposition false true)
          (set `self.Calibrated` true)
          (`KismetSystemLibrary.DelayUntilNextTick`)
          (`/Game/Blueprints/Turret/Tests/PC_Gyroscope.Flush` (`self.GyroscopeController`)))))))

(event `self.ReceiveTick`
  (params (DeltaSeconds :type "Float (single-precision)"))
  (bind _raycastplane (`self.RaycastPlane`))
  ;[1 0 0.01765] Tick
  (`|ExecutionSequence`
    (:`then_0`
      (if (`self.Calibrated`)
        (`|ExecutionSequence`
          (:`then_0`)
          (:`then_2`)
          (:`then_3`)
          (:`then_4`
            ;[1 0.3822 0.442] Reference Directions
            (for (_array_element _array_index) (`self.ReferenceDirections`) :!label _label
              (bind _returnvalue (`self.K2_GetActorLocation` (`|GetArrayItem` (`self.CalibrationTargets`) _array_index)))
              (`KismetSystemLibrary.DrawDebugLine` _returnvalue (+ (* (* _array_element 5000.0) -1.0) _returnvalue) (struct :`R` 1.0 :`G` 0.01685 :`A` 1.0) 0.0 2.0)))
          (:`then_5`)
          (:`then_6`
            (bind _hitpoint (`self.Raycast Against Plane` (`self.GetActorUpVector` _raycastplane) (`self.K2_GetActorLocation` _raycastplane) 0.0 (`self.K2_GetActorLocation`) (`/Game/Blueprints/Turret/Tests/PC_Gyroscope.PointerDirection` (`self.GyroscopeController`))))
            (`KismetSystemLibrary.DrawDebugSphere` _hitpoint 20.0 12 (struct :`R` 1.0 :`G` 0.00692 :`A` 1.0) 0.0 5.0)
            ;[0.5037 1 0.4594] Cursor
            (`KismetSystemLibrary.DrawDebugLine` (`self.K2_GetActorLocation`) _hitpoint (struct :`R` 0.41886 :`G` 1.0 :`B` 0.178601 :`A` 1.0) 0.0 5.0)))
        (else
          (`|ExecutionSequence`
            (:`then_0`)
            (:`then_1`
              (goto _label))
            (:`then_2`)))))
    (:`then_1`
      (`self.K2_SetActorRotation` (`/Game/Blueprints/Turret/Tests/PC_Gyroscope.TurretRotation` (`self.GyroscopeController`))))))

(fn `ComputeAverageDistanceBetweenPoints`
  (params (vectors :type "Array of Vector Structure"))
  (returns (AveragePoint :type "Vector Structure") (AverageDistanceToAveragePoint :type "Float (double-precision)"))
  (locals (Sum :type "Vector Structure") (DistanceSum :type "Float (double-precision)") (DistanceSumCount :type Integer) (averagePosition :type "Vector Structure"))
  (bind _returnvalue (`KismetArrayLibrary.Array_Length` vectors))
  (for _array_element vectors
    (set `local.Sum` (+ _array_element (`local.Sum`))))
  (bind _output_get (set `local.averagePosition` (/ (`local.Sum`) _returnvalue)))
  (for _array_element_2 vectors
    (set `local.DistanceSum` (+ (`KismetMathLibrary.Vector_Distance` _array_element_2 _output_get) (`local.DistanceSum`))))
  (return _output_get (/ (`local.DistanceSum`) _returnvalue)))

(fn `FindTurretPosition`
  (returns (TurretPosition :type "Vector Structure"))
  (locals (AveragePoint :type "Vector Structure") (AllHitPoints :type "Array of Vector Structure") (loopIndex :type "Vector2D Structure") (LastAverageDistance :type "Float (double-precision)" :default 1100000000.0) (CurrentAverageDistance :type "Float (double-precision)" :default 1000000000.0) (t :type "Float (double-precision)" :default 200.0) (iterations :type Integer))
  (bind _raycastplane (`self.RaycastPlane`))
  (bind _returnvalue (< (`local.iterations`) 10000))
  ;[1 0.6739 0.5157] While the average distance between the lines is decreasing
  (while (and (<= (`local.CurrentAverageDistance`) (`local.LastAverageDistance`)) _returnvalue)
    (`/Engine/EditorBlueprintResources/StandardMacros.IncrementInt` (`local.iterations`)
      (:`  `
        (bind _returnvalue_2 (+ (stale _output_get) 5.0))
        ;[1 0.5116 0.3568] March along Planes
        (bind _output_get (set `local.t` _returnvalue_2))
        (`KismetSystemLibrary.PrintString` (`KismetStringLibrary.Concat_StrStr` "t : " (`KismetStringLibrary.Conv_DoubleToString` _returnvalue_2)) true true (struct :`R` 0.105076 :`G` 0.406284 :`B` 1.0 :`A` 1.0) 20.0)
        (`KismetArrayLibrary.Array_Clear` (`local.AllHitPoints`))
        (for (_array_element _array_index) (`self.ReferenceDirections`)
          ;[1 0.4488 0.2698] Compute all 5 hit points on plane
          (bind _hitpoint (`self.Raycast Against Plane` (* (`self.GetActorUpVector` _raycastplane) -1.0) (`self.K2_GetActorLocation` _raycastplane) (* (`local.t`) -1.0) (`self.K2_GetActorLocation` (`|GetArrayItem` (`self.CalibrationTargets`) _array_index)) (* _array_element -1.0)))
          (`KismetArrayLibrary.Array_Add` (`local.AllHitPoints`) _hitpoint)
          (`|ExecutionSequence`))
        ;[0.375 0.2843 0.2441] Compute average distance between points on plane
        (bind (_averagepoint _averagedistancetoaveragepoint) (`self.ComputeAverageDistanceBetweenPoints` (`local.AllHitPoints`)))
        (set `local.LastAverageDistance` (`local.CurrentAverageDistance`))
        (set `local.CurrentAverageDistance` _averagedistancetoaveragepoint)
        (bind _output_get_2 (set `local.AveragePoint` _averagepoint))
        (`KismetSystemLibrary.DrawDebugSphere` _output_get_2 20.0 12 (struct :`R` 1.0 :`G` 1.0 :`B` 1.0 :`A` 1.0) 5.0 1.0))))
  (if _returnvalue
    (return (`local.AveragePoint`))
    (else
      (`KismetSystemLibrary.PrintString` "bug de salopard ça a failli exploser !" true true (struct :`R` 1.0 :`B` 0.029284 :`A` 1.0) 100.0))))

(fn `Raycast Against Plane`
  (params (PlaneNormal :type "Vector Structure") (PlaneStartPoint :type "Vector Structure") (PlaneOffsetAlongNormal :type "Float (double-precision)") (RayStart :type "Vector Structure") (RayDirection :type "Vector Structure"))
  (returns (HitPoint :type "Vector Structure"))
  (bind _returnvalue (`KismetMathLibrary.Normal` RayDirection))
  (bind _returnvalue_2 (`KismetMathLibrary.Normal` PlaneNormal))
  (bind _returnvalue_3 (* (/ (`KismetMathLibrary.Dot_VectorVector` _returnvalue_2 (- RayStart (+ PlaneStartPoint (* _returnvalue_2 PlaneOffsetAlongNormal)))) (`KismetMathLibrary.Dot_VectorVector` _returnvalue _returnvalue_2)) -1.0))
  (if (not (< _returnvalue_3 0.0))
    (`KismetSystemLibrary.PrintString` "no hit in front of line" true true (struct :`R` 1.0 :`G` 0.415181 :`B` 0.455003 :`A` 1.0)))
  (return (+ RayStart (* _returnvalue_3 _returnvalue))))

(fn `UserConstructionScript`)