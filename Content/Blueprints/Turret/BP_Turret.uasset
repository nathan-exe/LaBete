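; Player turret that fires repeated explosive shots at a world-space pointer to damage ghosts, initializing an Arduino gun interface through its gyroscope controller.
; A gated repeat macro drives each shot, applying sphere-overlap damage at a randomly scattered point with explosion VFX and pitch-shifted sound.
; Sustained fire widens spread and lengthens shot delay until StopShooting resets the shot count.
; Orbiting cursor triangles show the smoothed spread plus hit radius.
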(event `self.ReceiveTick`
  (params (DeltaSeconds :type "Float (single-precision)"))
  ;[1 0 0] Tick
  (`|ExecutionSequence`
    (:`then_0`
      (bind _output_get (set `self.CurrentSpreadRadius` (`KismetMathLibrary.FInterpTo` (stale _output_get) (`self.ComputeSpreadRadius`) DeltaSeconds (`self.SpreadReactionSpeed`)))))
    (:`then_1`
      (`self.UpdateCursorVisuals`))))

(event `self.ReceiveBeginPlay`
  (bind _ac_turretgyroscopecontroller (`self.AC_TurretGyroscopeController`))
  ;[1 0.04223 0] BeginPlay
  (`|ExecutionSequence`
    (:`then_0`
      ;[0.7188 0.3647 0.2928] Init Arduino
      (set `/Game/Blueprints/Turret/AC_TurretGyroscopeController.Arduino` (`self.AC_PhysicalGunControllerInterface`) _ac_turretgyroscopecontroller)
      (`/Game/Blueprints/Turret/AC_TurretGyroscopeController.init arduino` _ac_turretgyroscopecontroller))
    (:`then_1`
      ;[0.3058 0.7016 1] Harvest scene references
      (set `self.CursorSprites` (`|MakeArray` (`self.Triangle3`) (`self.Triangle1`) (`self.Triangle`) (`self.Triangle2`) :!type "SceneComponent Object Reference")))))

(event `SetPointerPosition`
  (params (WorldPos :type "Vector Structure"))
  ;[1 0 0] Set Pointer Position
  (`SceneComponent.K2_SetWorldLocation` (`self.Pointer`) (`KismetMathLibrary.MakeVector` (.x WorldPos) (.y WorldPos) 10.0) false false))

(event `Shoot`
  (bind _turretshot (`self.TurretShot`))
  ;[1 0 0] Shoot
  (`self.repeat` (`self.delayBetweenShots`) :!label _label
    (:`loop`
      (`/Engine/EditorBlueprintResources/StandardMacros.IncrementInt` (`self.CurrentShotID`)
        (:`  `
          (`|ExecutionSequence`
            (:`then_0`
              ;[0.4417 0.8694 1] Get all hit actors
              (bind _newparam (`self.ComputeHitLocation`))
              (bind _outactors (`KismetSystemLibrary.SphereOverlapActors` _newparam (`SphereComponent.SphereRadius` (`self.Sphere`)) (`|MakeArray` "ObjectTypeQuery2" "ObjectTypeQuery3" :!type "EObjectTypeQuery Enum")))
              (for _array_element _outactors
                ;[1 0.6389 0.9805] Damage ghosts
                (bind _asbp_ghost (cast `/Game/Blueprints/Ghost/BP_Ghost` _array_element))
                (`GameplayStatics.ApplyDamage` _asbp_ghost 1.0 null null "/Script/Engine.DamageType")))
            (:`then_1`
              ;[0.3585 0.6536 1] VFX
              (`NiagaraFunctionLibrary.SpawnSystemAtLocation` "/Game/Art/vfx/explosion.explosion" _newparam (struct) (1.0 1.0 1.0) true true "AutoRelease"))
            (:`then_2`
              ;[0.3215 0.111 0.3281 0.663] Sound
              (`AudioParameterControllerInterface.SetFloatParameter` _turretshot "ShotPitch" (* 0.1 (`self.CurrentShotID`)))
              (`AudioComponent.Play` _turretshot 0.0))))))))

(event `StopShooting`
  ;[1 0.02903 0] Cancel Shoot
  (set `self.CurrentShotID` 0)
  (goto _label :!via `Stop`))

(event `UpdateCursorVisuals`
  (bind _cursorsprites (`self.CursorSprites`))
  ;[1 0.07239 0.1022] UpdateCursorVisuals
  ;[0.4972 0.6651 1] Cursor Triangles
  (for (_array_element _array_index) _cursorsprites
    (bind _returnvalue (+ (* (/ (`KismetMathLibrary.Conv_IntToDouble` _array_index) (`KismetMathLibrary.Conv_IntToDouble` (`KismetArrayLibrary.Array_Length` _cursorsprites))) 360.0) (* (`KismetSystemLibrary.GetGameTimeInSeconds`) 90.0)))
    (`SceneComponent.K2_SetRelativeLocationAndRotation` _array_element (* (`KismetMathLibrary.MakeVector` (`KismetMathLibrary.DegCos` _returnvalue) 0.0 (`KismetMathLibrary.DegSin` _returnvalue)) (+ (`self.CurrentSpreadRadius`) (`SphereComponent.SphereRadius` (`self.Sphere`)))) (`KismetMathLibrary.MakeRotator` 0.0 (+ _returnvalue 90.0)) false false)))

(fn `ComputeHitLocation`
  (returns (NewParam :type "Vector Structure"))
  (return (+ (`SceneComponent.K2_GetComponentLocation` (`self.Pointer`)) (* (* (`KismetMathLibrary.RandomUnitVector`) (1.0 1.0 0.0)) (`self.ComputeSpreadRadius`)))))

(fn `UserConstructionScript`)