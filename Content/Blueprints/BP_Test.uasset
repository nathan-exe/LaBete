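; Test actor that links the game to an Arduino over a serial port, sending LedIntensity as a float every Tick.
; BeginPlay loops over port and baud ranges but always opens fixed port 3 at 9600, without breaking on success, printing results.
; Tick destroys the actor if the valid port is not open; EndPlay closes it.
; Unconnected nodes would read floats to drive PointLight intensity and flush the port.
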(event `self.ReceiveEndPlay`
  (params (EndPlayReason :type "EEndPlayReason Enum" :default "Destroyed"))
  (bind _arduinoport (`self.ArduinoPort`))
  ;[1 0.5088 0.467] Close Port
  (`/Engine/EditorBlueprintResources/StandardMacros.IsValid` _arduinoport
    (:`Is Valid`
      (`SerialCom.Close` _arduinoport))))

(event `self.ReceiveBeginPlay`
  (bind _arduinoport (`self.ArduinoPort`))
  (`|ExecutionSequence`
    (:`then_0`
      ;[0.7142 1 0.4643] find serial port
      (for _ (range 256)
        (for _ (`|MakeArray` 300 600 750 1200 2400 9600 19200)
          (bind (_bopened _returnvalue) (`SerialCom.OpenComPort` 3))
          (if _bopened
            (set `self.ArduinoPort` _returnvalue)
            (bind _returnvalue_2 (`KismetStringLibrary.Concat_StrStr` "serial port opening success : " (`KismetStringLibrary.Conv_BoolToString` _bopened)))
            (`KismetSystemLibrary.PrintString` _returnvalue_2 true true (struct :`R` 0.104774 :`G` 1.0 :`A` 1.0))
            (else
              (`KismetSystemLibrary.PrintString` _returnvalue_2 true true (struct :`R` 1.0 :`G` 0.099982 :`A` 1.0) 1.0))))))
    (:`then_1`
      ;[0.3284 1 0.3075] Print port info
      (`/Engine/EditorBlueprintResources/StandardMacros.IsValid` _arduinoport
        (:`Is Valid`
          (`KismetSystemLibrary.PrintString` (`KismetStringLibrary.Concat_StrStr` "Found Port with id : " (`KismetStringLibrary.Conv_IntToString` (`SerialCom.GetPort` _arduinoport)) " and baud rate : " (`KismetStringLibrary.Conv_IntToString` (`SerialCom.GetBaud` _arduinoport))) true true (struct :`G` 1.0 :`B` 0.069727 :`A` 1.0) 10.0))
        (:`Is Not Valid`
          (`KismetSystemLibrary.PrintString` "Couldn't open any port !!!" true true (struct :`R` 1.0 :`B` 0.05106 :`A` 1.0) 10.0))))))

(event `self.ReceiveTick`
  (params (DeltaSeconds :type "Float (single-precision)"))
  (bind _arduinoport (`self.ArduinoPort`))
  (`|ExecutionSequence`
    (:`then_0`
      (`/Engine/EditorBlueprintResources/StandardMacros.IsValid` _arduinoport
        (:`Is Valid`
          (if (`SerialCom.IsOpened` _arduinoport)
            (`SerialCom.WriteFloat` (`self.ArduinoPort`) (`self.ledIntensity`))
            (else
              (`KismetSystemLibrary.PrintString` "No Serial Port !!" true true (struct :`R` 1.0 :`G` 0.018015 :`A` 1.0) 10.0)
              (`self.K2_DestroyActor`))))))))

(fn `UserConstructionScript`)