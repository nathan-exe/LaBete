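; Shooter cursor Blueprint that repositions itself from a mouse XY axis input.
; Its Moove event prints a debug string, remaps X and Y toward 1920x1080 ranges and sets the location at zero Z, ignoring MapBounds.
; The custom remap float graph holds a linear formula that is left unconnected, adding D where a standard remap adds C.
; Shoot is an empty stub.
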(event `self.ReceiveBeginPlay`)

(event `Moove`
  (params (`Mouse x y axis` :type "Vector Structure") (`Map bounds` :type "LevelBounds Object Reference"))
  (bind (_x _y) (`KismetMathLibrary.BreakVector2D` (`KismetMathLibrary.Conv_VectorToVector2D` `Mouse x y axis`)))
  (`KismetSystemLibrary.PrintString` "Pitié bouge")
  (`self.K2_SetActorLocation` (`KismetMathLibrary.MakeVector` (`self.remap float` _x -800.0 800.0 0.0 1920.0) (`self.remap float` _y -450.0 450.0 0.0 1080.0))))

(event `Shoot`)

(fn `UserConstructionScript`)