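; BP_Shooter is a player-controlled shooting cursor that targets BP_Ghost actors.
; Enhanced Input moves the actor by the raw cursor input while CanMove is set, without sweep or delta-time scaling.
; While CanShoot is set, shooting runs a sphere trace for Pawns at its location and draws a red debug sphere.
; A BP_Ghost hit triggers ApplyDamage, though no damaged actor is shown wired to it.
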(event `EnhancedInput|/Game/Input/Turret/IA_MoveTurretCursor`
  (params (ActionValue :type "Vector2D Structure") (ElapsedSeconds :type "Float (double-precision)") (TriggeredSeconds :type "Float (double-precision)") (InputAction :type "InputAction Object Reference" :default "/Game/Input/Turret/IA_MoveTurretCursor.IA_MoveTurretCursor"))
  (:`Triggered`
    (if (`self.CanMove`)
      (`self.K2_SetActorLocation` (+ ActionValue (`self.K2_GetActorLocation`))))))

(event `EnhancedInput|/Game/Input/Turret/IA_Shoot`
  (params (ActionValue :type Boolean) (ElapsedSeconds :type "Float (double-precision)") (TriggeredSeconds :type "Float (double-precision)") (InputAction :type "InputAction Object Reference" :default "/Game/Input/Turret/IA_Shoot.IA_Shoot"))
  (bind _returnvalue (`self.K2_GetActorLocation`))
  (:`Triggered`
    (if (`self.CanShoot`)
      (bind (_outhit _returnvalue_2) (`KismetSystemLibrary.SphereTraceSingleForObjects` _returnvalue _returnvalue 50.0 (`|MakeArray` "ObjectTypeQuery3" :!type "EObjectTypeQuery Enum")))
      (`KismetSystemLibrary.DrawDebugSphere` _returnvalue 50.0 12 (struct :`R` 1.0 :`B` 0.003423 :`A` 1.0) 1.0)
      (if _returnvalue_2
        (cast `/Game/Blueprints/Ghost/BP_Ghost` (`.HitActor` (`GameplayStatics.BreakHitResult` _outhit)))
        (`GameplayStatics.ApplyDamage` null 1.0)))))

(fn `UserConstructionScript`)